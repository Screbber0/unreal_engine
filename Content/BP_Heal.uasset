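; BP_Heal is a single-use health pickup that heals the third-person character when it overlaps the Box component.
; It reads CurrentHealth from BP_GameInstance and heals by calling ApplyDamage with a negative value.
; The heal is a fixed amount, reduced near full health to only the missing portion up to 100, and the actor then destroys itself.
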(event OnComponentBeginOverlap(Box)
  (params (OverlappedComponent :type Primitive%20Component%20Object%20Reference) (OtherActor :type Actor%20Object%20Reference) (OtherComp :type Primitive%20Component%20Object%20Reference) (OtherBodyIndex :type Integer) (bFromSweep :type Boolean) (SweepResult :type Hit%20Result%20Structure%20%28by%20ref%29))
  (bind _asbp_third_person_character (Utilities|Casting|CastToBP_ThirdPersonCharacter OtherActor))
  (bind _asbp_game_instance (Utilities|Casting|CastToBP_GameInstance (Game|GetGameInstance)))
  (if (> (Variables|/Game/BP_GameInstance.BP_GameInstance_C|GetCurrent%20Health _asbp_game_instance) 8e+01)
    (Game|Damage|ApplyDamage _asbp_third_person_character (* (- 1e+02 (Variables|/Game/BP_GameInstance.BP_GameInstance_C|GetCurrent%20Health _asbp_game_instance)) -1.0) 0 0)
    (else
      (Game|Damage|ApplyDamage _asbp_third_person_character -2e+01 0 0)))
  (Actor|DestroyActor))

(event EventBeginPlay)

(event Collision|EventActorBeginOverlap
  (params (OtherActor :type Actor%20Object%20Reference)))

(event EventTick
  (params (DeltaSeconds :type Float%20%28single-precision%29)))

(fn ConstructionScript)