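; BP_Room is an actor that procedurally builds an open-topped box room from instanced cube meshes.
; GenerateRoom fills a floor grid and four walls with Cube instances in local space, spaced by MeshLength and sized by per-axis mesh counts.
; The construction script builds it from the current counts.
; BeginPlay randomizes the counts and generates again, without clearing existing instances.
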(event EventBeginPlay
  (Variables|Default|SetNumberMeshesX (Math|Random|RandomIntegerinRange 20 40))
  (Variables|Default|SetNumberMeshesY (Math|Random|RandomIntegerinRange 20 40))
  (Variables|Default|SetNumberMeshesZ (Math|Random|RandomIntegerinRange 5 10))
  (CallFunction|GenerateRoom))

(event Collision|EventActorBeginOverlap
  (params (OtherActor :type Actor%20Object%20Reference)))

(event EventTick
  (params (DeltaSeconds :type Float%20%28single-precision%29)))

(fn ConstructionScript
  (CallFunction|GenerateRoom))

(fn GenerateRoom
  (CallFunction|GenerateFloor)
  (CallFunction|GenerateFrontWall)
  (CallFunction|GenerateBackWall)
  (CallFunction|GenerateRightWall)
  (CallFunction|GenerateLeftWall))

(fn GenerateFloor
  (bind _meshlength (Variables|Default|GetMeshLength))
  (for _index (range 0 (- (Variables|Default|GetNumberMeshesX) 1))
    (for _index_2 (range 0 (- (Variables|Default|GetNumberMeshesY) 1))
      (Components|InstancedStaticMesh|AddInstance (Variables|Default|GetCube) (Math|Transform|MakeTransform (Math|Vector|MakeVector (* _index _meshlength) (* _index_2 _meshlength) 0.0)) false))))

(fn GenerateFrontWall
  (bind _meshlength (Variables|Default|GetMeshLength))
  (for _index (range 0 (- (Variables|Default|GetNumberMeshesY) 1))
    (for _index_2 (range 0 (Variables|Default|GetNumberMeshesZ))
      (Components|InstancedStaticMesh|AddInstance (Variables|Default|GetCube) (Math|Transform|MakeTransform (Math|Vector|MakeVector (* _meshlength (Variables|Default|GetNumberMeshesX)) (* _index _meshlength) (* _index_2 _meshlength))) false))))

(fn GenerateBackWall
  (bind _meshlength (Variables|Default|GetMeshLength))
  (for _index (range 0 (- (Variables|Default|GetNumberMeshesY) 1))
    (for _index_2 (range 0 (Variables|Default|GetNumberMeshesZ))
      (Components|InstancedStaticMesh|AddInstance (Variables|Default|GetCube) (Math|Transform|MakeTransform (Math|Vector|MakeVector 0.0 (* _index _meshlength) (* _index_2 _meshlength))) false))))

(fn GenerateRightWall
  (bind _meshlength (Variables|Default|GetMeshLength))
  (for _index (range 0 (- (Variables|Default|GetNumberMeshesX) 1))
    (for _index_2 (range 0 (Variables|Default|GetNumberMeshesZ))
      (Components|InstancedStaticMesh|AddInstance (Variables|Default|GetCube) (Math|Transform|MakeTransform (Math|Vector|MakeVector (* _index _meshlength) (* _meshlength (Variables|Default|GetNumberMeshesY)) (* _index_2 _meshlength))) false))))

(fn GenerateLeftWall
  (bind _meshlength (Variables|Default|GetMeshLength))
  (for _index (range 0 (- (Variables|Default|GetNumberMeshesX) 0))
    (for _index_2 (range 0 (Variables|Default|GetNumberMeshesZ))
      (Components|InstancedStaticMesh|AddInstance (Variables|Default|GetCube) (Math|Transform|MakeTransform (Math|Vector|MakeVector (* _index _meshlength) 0.0 (* _index_2 _meshlength))) false))))